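; BP_ASPawnBullet is a bullet actor that damages ASCharacter targets through their health component.
; On overlap it applies fixed damage to a character and destroys itself, passes through any ASPawn, and destroys itself on any other actor.
; The hit handler mirrors this logic but tests SelfActor, the bullet itself, for the character class while still looking up health on OtherActor.
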(event Custom|OnActorHit_Event
  (params (SelfActor :type Actor%20Object%20Reference) (OtherActor :type Actor%20Object%20Reference) (NormalImpulse :type Vector) (Hit :type Hit%20Result%20Structure%20%28by%20ref%29))
  (if (Class|GameplayStatics|ObjectIsA SelfActor "/Script/ArenaShooter.ASCharacter")
    (Class|ASHealthComponent|Damage (Class|ASHealthComponent|FindHealthComponent OtherActor) 1e+01 self 0.0 "0, 0, 0" "0, 0, 0")
    (Actor|DestroyActor :!label _label)
    (elif (not (Class|GameplayStatics|ObjectIsA OtherActor "/Script/ArenaShooter.ASPawn"))
      (goto _label))))

(event EventBeginPlay)

(event Collision|EventActorBeginOverlap
  (params (OtherActor :type Actor%20Object%20Reference))
  (if (Class|GameplayStatics|ObjectIsA OtherActor "/Script/ArenaShooter.ASCharacter")
    (Class|ASHealthComponent|Damage (Class|ASHealthComponent|FindHealthComponent OtherActor) 1e+01 self 0.0 "0, 0, 0" "0, 0, 0")
    (Actor|DestroyActor :!label _label)
    (elif (not (Class|GameplayStatics|ObjectIsA OtherActor "/Script/ArenaShooter.ASPawn"))
      (goto _label))))

(event EventTick
  (params (DeltaSeconds :type Float%20%28single-precision%29)))

(fn ConstructionScript)