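; BP_BasicBullet is a weapon projectile Blueprint that reacts to what it overlaps.
; It ignores ASCharacter actors and destroys itself shortly after overlapping an ASDronePawn.
; Any other overlap sets its speed to zero, plays a miss sound, activates its Niagara effect and destroys it after a longer delay.
; The graph applies no damage itself, and its Hit, Tick and construction logic are empty.
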(event EventBeginPlay)

(event Collision|EventActorBeginOverlap
  (params (OtherActor :type Actor%20Object%20Reference))
  (if (not (Class|GameplayStatics|ObjectIsA OtherActor "/Script/ArenaShooter.ASCharacter"))
    (if (Class|GameplayStatics|ObjectIsA OtherActor "/Script/ArenaShooter.ASDronePawn")
      (Utilities|FlowControl|Delay 0.3)
      (Actor|DestroyActor)
      (else
        (Class|ASBasicBullet|SetSpeed 0.0)
        (Audio|PlaySoundatLocation "/Game/Sound/New-Sound/SOUND-MissShotV2_Cue.SOUND-MissShotV2_Cue" (Transformation|GetActorLocation) "0, 0, 0" 1.0 1.0 0.0 0 0 0 0)
        (Components|Activation|Activate (Variables|Default|GetNiagara) false)
        (Utilities|FlowControl|Delay 5.0)
        (Actor|DestroyActor)))))

(event EventTick
  (params (DeltaSeconds :type Float%20%28single-precision%29)))

(event Collision|EventHit
  (params (MyComp :type Primitive%20Component%20Object%20Reference) (Other :type Actor%20Object%20Reference) (OtherComp :type Primitive%20Component%20Object%20Reference) (bSelfMoved :type Boolean) (HitLocation :type Vector :default "0, 0, 0") (HitNormal :type Vector :default "0, 0, 0") (NormalImpulse :type Vector :default "0, 0, 0") (Hit :type Hit%20Result%20Structure%20%28by%20ref%29)))

(fn ConstructionScript)