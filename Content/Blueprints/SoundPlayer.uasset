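; SoundPlayer is an actor that plays the MusiqueGravitesseV1Cue music from BeginPlay and bends its pitch to follow global time dilation.
; Each Tick lerps the pitch multiplier toward the current dilation, dividing delta time by the dilation so the smoothing runs at real-time speed.
; PreviousFrameTime is reset to zero each Tick but never read here.
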(event EventBeginPlay
  (Audio|Components|Audio|Play (Variables|Default|GetMusique_Gravitesse_V1_Cue) 0.0))

(event Collision|EventActorBeginOverlap
  (params (OtherActor :type Actor%20Object%20Reference)))

(event EventTick
  (params (DeltaSeconds :type Float%20%28single-precision%29))
  (bind _musique_gravitesse_v1_cue (Variables|Default|GetMusique_Gravitesse_V1_Cue))
  (Audio|Components|Audio|SetPitchMultiplier _musique_gravitesse_v1_cue (Math|Float|Lerp (Variables|/Script/Engine.AudioComponent|GetPitchMultiplier _musique_gravitesse_v1_cue) (Class|GameplayStatics|GetGlobalTimeDilation) (* (* DeltaSeconds (/ 1.0 (Class|GameplayStatics|GetGlobalTimeDilation))) 3.0)))
  (Variables|Default|SetpreviousFrameTime 0.0))

(fn ConstructionScript)