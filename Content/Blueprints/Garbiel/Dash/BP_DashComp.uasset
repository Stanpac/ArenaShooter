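; BP_DashComp is a component that gives its owning ASCharacter a dash on Left Shift.
; It launches the character along the first-person camera's forward vector, switching to flying with no ground friction and lowered gravity.
; After a short delay it sets walking mode and hardcoded friction and gravity values, then clears the cooldown after another delay.
; A press during cooldown only prints a debug message.
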(event Input|KeyboardEvents|LeftShift
  (params (Key :type Key%20Structure))
  (:Pressed
    (bind _asascharacter (Utilities|Casting|CastToASCharacter (Components|GetOwner)))
    (if (Variables|Default|GetIsInCooldown)
      (Development|PrintString "DashInCooldown")
      (else
        (Pawn|Components|CharacterMovement|SetMovementMode (Variables|/Script/Engine.Character|GetCharacterMovement _asascharacter) "MOVE_Flying" 0)
        (Character|LaunchCharacter _asascharacter (* (Math|Vector|GetForwardVector (Variables|/Script/ArenaShooter.ASCharacter|Getm_FirstPersonCameraComponent _asascharacter)) (Variables|Default|GetDashPowerValue)) false false)
        (Variables|Default|SetIsInCooldown true)
        (Variables|/Script/Engine.CharacterMovementComponent|SetGroundFriction (Variables|/Script/Engine.Character|GetCharacterMovement _asascharacter) 0.0)
        (Variables|/Script/Engine.CharacterMovementComponent|SetGravityScale (Variables|/Script/Engine.Character|GetCharacterMovement _asascharacter) 1.0)
        (Utilities|FlowControl|Delay 0.7)
        (Pawn|Components|CharacterMovement|SetMovementMode (Variables|/Script/Engine.Character|GetCharacterMovement _asascharacter) "MOVE_Walking" 0)
        (Variables|/Script/Engine.CharacterMovementComponent|SetGroundFriction (Variables|/Script/Engine.Character|GetCharacterMovement _asascharacter) 8.0)
        (Variables|/Script/Engine.CharacterMovementComponent|SetGravityScale (Variables|/Script/Engine.Character|GetCharacterMovement _asascharacter) 4.0)
        (Utilities|FlowControl|Delay 1.0)
        (Variables|Default|SetIsInCooldown false)))))