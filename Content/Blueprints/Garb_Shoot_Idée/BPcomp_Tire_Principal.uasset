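; Primary fire component for BP_ASCharacter that fires a burst of plasma-sounding projectiles on the Shoot input.
; A press plays a camera shake and a shot sound, then starts a self-calling Again event with a short delay before each shot.
; Each shot spawns Shoot_Projectile at the character's location along the first-person camera's aim with slight random spread.
; ShootCount counts down the burst and resets when it reaches zero.
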(event Custom|Again!
  (if (> (Variables|Default|GetShootCount) 0)
    (Utilities|FlowControl|Delay 0.03)
    (Game|SpawnActorfromClass "/Game/Blueprints/Garb_Shoot_Idée/Shoot_Projectile.Shoot_Projectile_C" (Math|Transform|MakeTransform (.location (Transformation|GetActorTransform (stale Input|ActionEvents|InputActionShoot _asbp_ascharacter))) (Math|Rotator|MakeRotator 0.0 (+ (.pitch (Transformation|GetWorldRotation (Variables|/Script/ArenaShooter.ASCharacter|Getm_FirstPersonCameraComponent (stale Input|ActionEvents|InputActionShoot _asbp_ascharacter)))) (Math|Random|RandomFloatinRange -1.5 1.5)) (+ (.yaw (Transformation|GetWorldRotation (Variables|/Script/ArenaShooter.ASCharacter|Getm_FirstPersonCameraComponent (stale Input|ActionEvents|InputActionShoot _asbp_ascharacter)))) (Math|Random|RandomFloatinRange -1.5 1.5))) "1.000000,1.000000,1.000000") "Undefined" "MultiplyWithRoot" 0 0)
    (Audio|PlaySoundatLocation "/Game/Blueprints/Garb_Shoot_Idée/Son_TirePrincipal/Son_Tire/Piou_Plasma_Doom.Piou_Plasma_Doom" "0, 0, 0" "0, 0, 0" 1.0 1.0 0.0 0 0 0 0)
    (Math|Integer|DecrementInt (Variables|Default|GetShootCount)
      (:%20%20
        (CallFunction|Again!)))
    (else
      (Variables|Default|SetShootCount 10))))

(event Input|ActionEvents|InputActionShoot
  (params (Key :type Key%20Structure :default "None"))
  (:Pressed
    (bind _asbp_ascharacter (Utilities|Casting|CastToBP_ASCharacter (Components|GetOwner)))
    (Camera|PlayWorldCameraShake "/Game/Blueprints/Garb_Shoot_Idée/BP_Shoot_CameraShake.BP_Shoot_CameraShake_C" (.location (Transformation|GetActorTransform _asbp_ascharacter)) 0.0 5e+02)
    (Audio|PlaySoundatLocation "/Game/Sound/SOUND_Shot_Drone.SOUND_Shot_Drone" "0, 0, 0" "0, 0, 0" 1.0 1.0 0.0 0 0 0 0)
    (if (> (Variables|Default|GetShootCount) 0)
      (Utilities|FlowControl|Delay 0.03)
      (Game|SpawnActorfromClass "/Game/Blueprints/Garb_Shoot_Idée/Shoot_Projectile.Shoot_Projectile_C" (Math|Transform|MakeTransform (.location (Transformation|GetActorTransform _asbp_ascharacter)) (Math|Rotator|MakeRotator 0.0 (+ (.pitch (Transformation|GetWorldRotation (Variables|/Script/ArenaShooter.ASCharacter|Getm_FirstPersonCameraComponent _asbp_ascharacter))) (Math|Random|RandomFloatinRange -1.5 1.5)) (+ (.yaw (Transformation|GetWorldRotation (Variables|/Script/ArenaShooter.ASCharacter|Getm_FirstPersonCameraComponent _asbp_ascharacter))) (Math|Random|RandomFloatinRange -1.5 1.5))) "1.000000,1.000000,1.000000") "Undefined" "MultiplyWithRoot" 0 0)
      (Audio|PlaySoundatLocation "/Game/Blueprints/Garb_Shoot_Idée/Son_TirePrincipal/Son_Tire/Piou_Plasma_Doom.Piou_Plasma_Doom" "0, 0, 0" "0, 0, 0" 1.0 1.0 0.0 0 0 0 0)
      (Math|Integer|DecrementInt (Variables|Default|GetShootCount)
        (:%20%20
          (CallFunction|Again!)))
      (else
        (Variables|Default|SetShootCount 10)))))